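; GravPlayerController is a player controller that lets the player toggle between push and pull gravity colours.
; On BeginPlay it caches the GravGamemode reference.
; Pressing the Switch input flips the GravColours state between ColourPush and ColourPull, then passes the new value to the game mode through CallSwitch.
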(event EventBeginPlay
  (bind _asgrav_gamemode (Utilities|Casting|CastToGravGamemode (Game|GetGameMode)))
  (Variables|Default|SetGGamemode _asgrav_gamemode))

(event EventTick
  (params (DeltaSeconds :type Float%20%28single-precision%29)))

(event Input|ActionEvents|InputActionSwitch
  (params (Key :type Key%20Structure :default "AnyKey"))
  ;[1 1 1] Switch
  (:Pressed
    (switch Utilities|FlowControl|Switch|SwitchonColours (Variables|Default|GetGravColours)
      (:NewEnumerator0
        (Variables|Default|SetGravColours "NewEnumerator1"))
      (:NewEnumerator1
        (Variables|Default|SetGravColours "NewEnumerator0")))
    (Default|CallSwitch (Variables|Default|GetGGamemode) (Variables|Default|GetGravColours))))

(fn ConstructionScript)