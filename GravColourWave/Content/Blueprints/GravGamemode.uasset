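; Game mode that tracks a timed noodle-collecting run and ends it when time or noodles run out.
; BeginPlay counts the PotOfNoodles actors and starts the timer at TimeMax, which Tick counts down while enabled.
; PickUpNoodles updates the remaining and collected counts.
; Gameover stops the timer, saves score and elapsed time to the PersistentData game instance, then opens EndLevel; a timeout first sets Timer to -10.
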(event Custom|PickUpNoodles
  (bind _result (Math|Integer|DecrementInt (Variables|Default|GetNoodlesLeft))
    (:%20%20
      (Math|Integer|IncrementInt (Variables|Default|GetNoodlesCollected)
        (:%20%20
          (if (<= _result 0)
            (Development|PrintString "GameOver" true true "(R=1.000000,G=0.000000,B=0.052548,A=1.000000)")
            (CallFunction|Gameover)))))))

(event EventBeginPlay
  (bind _outactors (Actor|GetAllActorsOfClass "/Game/Blueprints/PotOfNoodles.PotOfNoodles_C"))
  (Variables|Default|SetNoodlesLeft (Utilities|Array|Length _outactors))
  (Variables|Default|SetTimer (Variables|Default|GetTimeMax)))

(event EventTick
  (params (DeltaSeconds :type Float%20%28single-precision%29))
  (if (Variables|Default|GetisTimerEnabled)
    (bind _output_get (Variables|Default|SetTimer (- (Variables|Default|GetTimer) DeltaSeconds)))
    (if (<= _output_get 0.0)
      (Variables|Default|SetTimer -1e+01)
      (CallFunction|Gameover))))

(fn ConstructionScript)

(fn Gameover
  (Variables|Default|SetisTimerEnabled false)
  (bind _aspersistent_data (Utilities|Casting|CastToPersistentData (Game|GetGameInstance))
    (:then
      (Default|SetNewTimeandScore _aspersistent_data (Variables|Default|GetNoodlesCollected) (- (Variables|Default|GetTimeMax) (Variables|Default|GetTimer)))
      (Game|OpenLevel(byName) "EndLevel"))
    (:CastFailed
      (Development|PrintString "No pData"))))