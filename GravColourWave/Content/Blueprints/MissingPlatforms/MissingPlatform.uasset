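; MissingPlatform is a colour-keyed platform that is solid only while the active gravity colour matches its own Colour.
; On BeginPlay it reads the current colour from GravPlayerController and binds Switch to the GravGamemode's switch event.
; UpdateMatCol swaps between solid and missing materials, toggles collision, and tints EmissiveColour red for push or blue for pull.
; The construction script previews it as if ColourPush were active.
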(event Custom|Switch
  (params (Colour :type Colours%20Enum))
  (CallFunction|UpdateMatCol Colour))

(event Collision|EventActorBeginOverlap
  (params (OtherActor :type Actor%20Object%20Reference)))

(event EventTick
  (params (DeltaSeconds :type Float%20%28single-precision%29)))

(event EventBeginPlay
  (bind _asgrav_player_controller (Utilities|Casting|CastToGravPlayerController (Game|GetPlayerController 0))
    (:then
      (CallFunction|UpdateMatCol (Variables|/Game/Blueprints/GravPlayerController.GravPlayerController_C|GetGravColours _asgrav_player_controller)))
    (:CastFailed
      _))
  (bind _asgrav_gamemode (Utilities|Casting|CastToGravGamemode (Game|GetGameMode)))
  (EventDispatchers|BindEventtoSwitch _asgrav_gamemode (delegate Custom|Switch)))

(fn ConstructionScript
  (CallFunction|UpdateMatCol "NewEnumerator0"))

(fn UpdateMatCol
  (params (CurrentColour :type Colours%20Enum))
  (bind _staticmesh (Variables|Default|GetStaticMesh))
  (bind _staticmesh_2 (Variables|Default|GetStaticMesh))
  (if (Utilities|Enum|Equal(Enum) CurrentColour (Variables|Default|GetColour))
    (Rendering|Material|SetMaterial _staticmesh_2 0 "/Game/Art/White_Mat.White_Mat")
    (Rendering|Material|SetMaterial _staticmesh_2 1 "/Game/Art/GravityModule_Mat.GravityModule_Mat")
    (Collision|SetCollisionEnabled _staticmesh "QueryAndPhysics")
    (else
      (Rendering|Material|SetMaterial _staticmesh_2 0 "/Game/Art/MissingPlatform_Inst.MissingPlatform_Inst")
      (Rendering|Material|SetMaterial _staticmesh_2 1 "/Game/Art/MissingPlatform_Inst.MissingPlatform_Inst")
      (Collision|SetCollisionEnabled _staticmesh "NoCollision")))
  (Rendering|Material|SetVectorParameterValueonMaterials (Variables|Default|GetStaticMesh) "EmissiveColour" (Utilities|Select :Index (Variables|Default|GetColour) :NewEnumerator0 "1.000000,0,0" :NewEnumerator1 "0,0.000000,1.000000")))