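; PersistentData holds the latest run's player name, noodle score and time, and persists a score history to disk.
; Setter functions store the recent values, then SetScores loads the "scores" slot, appends them to parallel Times, Names and Noodles arrays, and saves.
; Both SetScores and SaveGameSlot write by creating a fresh GravSaveGame, copying the arrays into it and overwriting the slot.
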(fn SetNewTimeandScore
  (params (Noodles :type Integer) (Times :type Float%20%28single-precision%29))
  (Variables|Default|SetRecentNoodlesScore Noodles)
  (Variables|Default|SetRecentTime Times))

(fn SetNewName
  (params (name :type Text))
  (Variables|Default|SetrecentName name))

(fn SetScores
  (bind _returnvalue (SaveGame|LoadGamefromSlot "scores"))
  (bind _asgrav_save_game (Utilities|Casting|CastToGravSaveGame _returnvalue)
    (:then
      (bind _output_get (Variables|Default|SetTimes (Variables|/Game/Blueprints/GravSaveGame.GravSaveGame_C|GetTimes _asgrav_save_game)))
      (bind _output_get_2 (Variables|Default|SetNames (Variables|/Game/Blueprints/GravSaveGame.GravSaveGame_C|GetNames _asgrav_save_game)))
      (bind _output_get_3 (Variables|Default|SetNoodles (Variables|/Game/Blueprints/GravSaveGame.GravSaveGame_C|GetNoodles _asgrav_save_game))))
    (:CastFailed
      _))
  (Utilities|Array|Add (Variables|Default|GetTimes) (Variables|Default|GetRecentTime))
  (Utilities|Array|Add (Variables|Default|GetNames) (Variables|Default|GetrecentName))
  (Utilities|Array|Add (Variables|Default|GetNoodles) (Variables|Default|GetRecentNoodlesScore))
  (bind _returnvalue_2 (SaveGame|CreateSaveGameObject "/Game/Blueprints/GravSaveGame.GravSaveGame_C"))
  (bind _asgrav_save_game_2 (Utilities|Casting|CastToGravSaveGame _returnvalue_2))
  (Variables|/Game/Blueprints/GravSaveGame.GravSaveGame_C|SetNames _asgrav_save_game_2 _output_get_2)
  (Variables|/Game/Blueprints/GravSaveGame.GravSaveGame_C|SetNoodles _asgrav_save_game_2 _output_get_3)
  (Variables|/Game/Blueprints/GravSaveGame.GravSaveGame_C|SetTimes _asgrav_save_game_2 _output_get)
  (SaveGame|SaveGametoSlot _returnvalue_2 "scores"))

(fn SaveGameSlot
  (bind _returnvalue (SaveGame|CreateSaveGameObject "/Game/Blueprints/GravSaveGame.GravSaveGame_C"))
  (bind _asgrav_save_game (Utilities|Casting|CastToGravSaveGame _returnvalue))
  (Variables|/Game/Blueprints/GravSaveGame.GravSaveGame_C|SetNames _asgrav_save_game (Variables|Default|GetNames))
  (Variables|/Game/Blueprints/GravSaveGame.GravSaveGame_C|SetNoodles _asgrav_save_game (Variables|Default|GetNoodles))
  (Variables|/Game/Blueprints/GravSaveGame.GravSaveGame_C|SetTimes _asgrav_save_game (Variables|Default|GetTimes))
  (SaveGame|SaveGametoSlot _returnvalue "scores"))