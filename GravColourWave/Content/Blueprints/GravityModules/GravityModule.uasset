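; Gravity module that pushes or pulls Pushable actors and the player, with its emissive colour showing red for push and blue for pull.
; Each tick it applies force to overlapping targets, radially from a sphere or along its up vector in a box, depending on IsRadial.
; The GravGamemode switch event flips its mode and material.
; Player overlap with either volume toggles the character's own gravity off on entry and on at exit.
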(event OnComponentBeginOverlap(Box)
  (params (OverlappedComponent :type Primitive%20Component%20Object%20Reference) (OtherActor :type Actor%20Object%20Reference) (OtherComp :type Primitive%20Component%20Object%20Reference) (OtherBodyIndex :type Integer) (bFromSweep :type Boolean) (SweepResult :type Hit%20Result%20Structure%20%28by%20ref%29))
  (bind _asgrav_first_person_character (Utilities|Casting|CastToGravFirstPersonCharacter OtherActor))
  (Default|ToggleGravity _asgrav_first_person_character false))

(event OnComponentBeginOverlap(Sphere)
  (params (OverlappedComponent :type Primitive%20Component%20Object%20Reference) (OtherActor :type Actor%20Object%20Reference) (OtherComp :type Primitive%20Component%20Object%20Reference) (OtherBodyIndex :type Integer) (bFromSweep :type Boolean) (SweepResult :type Hit%20Result%20Structure%20%28by%20ref%29))
  (bind _asgrav_first_person_character (Utilities|Casting|CastToGravFirstPersonCharacter OtherActor))
  (Default|ToggleGravity _asgrav_first_person_character false))

(event OnComponentEndOverlap(Sphere)
  (params (OverlappedComponent :type Primitive%20Component%20Object%20Reference) (OtherActor :type Actor%20Object%20Reference) (OtherComp :type Primitive%20Component%20Object%20Reference) (OtherBodyIndex :type Integer))
  (bind _asgrav_first_person_character (Utilities|Casting|CastToGravFirstPersonCharacter OtherActor))
  (Default|ToggleGravity _asgrav_first_person_character true))

(event OnComponentEndOverlap(Box)
  (params (OverlappedComponent :type Primitive%20Component%20Object%20Reference) (OtherActor :type Actor%20Object%20Reference) (OtherComp :type Primitive%20Component%20Object%20Reference) (OtherBodyIndex :type Integer))
  (bind _asgrav_first_person_character (Utilities|Casting|CastToGravFirstPersonCharacter OtherActor))
  (Default|ToggleGravity _asgrav_first_person_character true))

(event Custom|Switch
  (params (Colour :type Colours%20Enum))
  (Variables|Default|SetColour Colour)
  (CallFunction|UpdateMat))

(event EventBeginPlay
  (CallFunction|UpdateMat)
  (bind _asgrav_gamemode (Utilities|Casting|CastToGravGamemode (Game|GetGameMode)))
  (EventDispatchers|BindEventtoSwitch _asgrav_gamemode (delegate Custom|Switch)))

(event EventTick
  (params (DeltaSeconds :type Float%20%28single-precision%29))
  (if (Variables|Default|GetIsRadial)
    (CallFunction|PushPullRadial)
    (else
      (CallFunction|PushPullFlat))))

(fn ConstructionScript
  (CallFunction|UpdateMat))

(fn PushPullRadial
  (bind _sphere (Variables|Default|GetSphere))
  (for _array_element (Collision|GetOverlappingActors _sphere "/Game/Blueprints/Pushables/Pushable.Pushable_C" :!class /Script/Engine.PrimitiveComponent)
    ;[1 1 1] Pushable
    (bind _aspushable (Utilities|Casting|CastToPushable _array_element))
    (switch Utilities|FlowControl|Switch|SwitchonColours (Variables|Default|GetColour)
      (:NewEnumerator0
        (Physics|AddForce (Variables|/Game/Blueprints/Pushables/Pushable.Pushable_C|GetMesh _aspushable) (* (Math|Vector|GetForwardVector (Math|Rotator|FindLookatRotation (Transformation|GetActorLocation) (Transformation|GetActorLocation _aspushable))) (* (Variables|Default|GetPushStrength) (Variables|Default|GetbaseStrength))) "None" false))
      (:NewEnumerator1
        (Physics|AddForce (Variables|/Game/Blueprints/Pushables/Pushable.Pushable_C|GetMesh _aspushable) (* (Math|Vector|GetForwardVector (Math|Rotator|FindLookatRotation (Transformation|GetActorLocation _aspushable) (Transformation|GetActorLocation))) (* (Variables|Default|GetPullStrength) (Variables|Default|GetbaseStrength))) "None" false))))
  (for _array_element_2 (Collision|GetOverlappingActors _sphere "/Game/Blueprints/GravFirstPersonCharacter.GravFirstPersonCharacter_C" :!class /Script/Engine.PrimitiveComponent)
    ;[1 1 1] Player
    (bind _asgrav_first_person_character (Utilities|Casting|CastToGravFirstPersonCharacter _array_element_2))
    (switch Utilities|FlowControl|Switch|SwitchonColours (Variables|Default|GetColour)
      (:NewEnumerator0
        (Physics|AddForce (Variables|/Script/Engine.Character|GetCharacterMovement _asgrav_first_person_character) (* (Math|Vector|GetForwardVector (Math|Rotator|FindLookatRotation (Transformation|GetActorLocation) (Transformation|GetActorLocation _asgrav_first_person_character))) (* (Variables|Default|GetPushStrength) (Variables|Default|GetbaseStrength)))))
      (:NewEnumerator1
        (Physics|AddForce (Variables|/Script/Engine.Character|GetCharacterMovement _asgrav_first_person_character) (* (Math|Vector|GetForwardVector (Math|Rotator|FindLookatRotation (Transformation|GetActorLocation _asgrav_first_person_character) (Transformation|GetActorLocation))) (* (Variables|Default|GetPullStrength) (Variables|Default|GetbaseStrength))))))))

(fn UpdateMat
  (switch Utilities|FlowControl|Switch|SwitchonColours (Variables|Default|GetColour)
    (:NewEnumerator0
      (Rendering|Material|SetVectorParameterValueonMaterials (Variables|Default|GetMesh) "EmissiveColour" (Math|Conversions|ToVector(LinearColor) (Math|Color|MakeColor 1.0 0.0 0.0))))
    (:NewEnumerator1
      (Rendering|Material|SetVectorParameterValueonMaterials (Variables|Default|GetMesh) "EmissiveColour" (Math|Conversions|ToVector(LinearColor) (Math|Color|MakeColor 0.0 0.0 1.0))))))

(fn PushPullFlat
  (bind _box (Variables|Default|GetBox))
  (for _array_element (Collision|GetOverlappingActors _box "/Game/Blueprints/Pushables/Pushable.Pushable_C" :!class /Script/Engine.PrimitiveComponent)
    ;[1 1 1] Pushable
    (bind _aspushable (Utilities|Casting|CastToPushable _array_element))
    (switch Utilities|FlowControl|Switch|SwitchonColours (Variables|Default|GetColour)
      (:NewEnumerator0
        (Physics|AddForce (Variables|/Game/Blueprints/Pushables/Pushable.Pushable_C|GetMesh _aspushable) (* (Transformation|GetActorUpVector) (* (Variables|Default|GetPushStrength) (Variables|Default|GetbaseStrength))) "None" false))
      (:NewEnumerator1
        (Physics|AddForce (Variables|/Game/Blueprints/Pushables/Pushable.Pushable_C|GetMesh _aspushable) (* (Transformation|GetActorUpVector) (* (Variables|Default|GetPullStrength) (Variables|Default|GetbaseStrength) -1.0)) "None" false))))
  (for _array_element_2 (Collision|GetOverlappingActors _box "/Game/Blueprints/GravFirstPersonCharacter.GravFirstPersonCharacter_C" :!class /Script/Engine.PrimitiveComponent)
    ;[1 1 1] Player
    (bind _asgrav_first_person_character (Utilities|Casting|CastToGravFirstPersonCharacter _array_element_2))
    (switch Utilities|FlowControl|Switch|SwitchonColours (Variables|Default|GetColour)
      (:NewEnumerator0
        (Physics|AddForce (Variables|/Script/Engine.Character|GetCharacterMovement _asgrav_first_person_character) (* (Transformation|GetActorUpVector) (* (Variables|Default|GetPushStrength) (Variables|Default|GetbaseStrength)))))
      (:NewEnumerator1
        (Physics|AddForce (Variables|/Script/Engine.Character|GetCharacterMovement _asgrav_first_person_character) (* (Transformation|GetActorUpVector) (* (Variables|Default|GetPullStrength) (Variables|Default|GetbaseStrength) -1.0)))))))

(fn SetGravityVolumes
  (if (Variables|Default|GetIsRadial)
    (Variables|/Script/Engine.PrimitiveComponent|SetbGenerateOverlapEvents (Variables|Default|GetBox) false)
    (else
      (Variables|/Script/Engine.PrimitiveComponent|SetbGenerateOverlapEvents (Variables|Default|GetSphere) false))))